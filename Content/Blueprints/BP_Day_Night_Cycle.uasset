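; Day/night cycle Blueprint that animates the sun and sky, toggled with the T key.
; A FlipFlop plays or stops a timeline whose pitch and yaw tracks rotate the light source and refresh the sky sphere's sun direction at half play rate.
; BeginPlay converts system time to fractional hours, but both toggle branches reset that value to noon, with comments marking rewiring for real-time use.
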(event `self.ReceiveBeginPlay`
  (bind _returnvalue (`KismetMathLibrary.Now`))
  (`self.EnableInput` (`GameplayStatics.GetPlayerController` 0))
  (set `self.NewTime` (+ (`KismetMathLibrary.Conv_IntToDouble` (`KismetMathLibrary.GetHour` _returnvalue)) (/ (`KismetMathLibrary.Conv_IntToDouble` (`KismetMathLibrary.GetMinute` _returnvalue)) 60.0) (/ (`KismetMathLibrary.Conv_IntToDouble` (`KismetMathLibrary.GetSecond` _returnvalue)) 3600.0))) ; Connect to play if what to use system time
)

(event `Key|T`
  (params (Key :type "Key Structure"))
  (:`Pressed`
    (`/Engine/EditorBlueprintResources/StandardMacros.FlipFlop`
      (:`A`
        (`|ExecutionSequence`
          (:`then_0`
            (bind (_direction _sun_pitch _sun_yaw) (`Timeline|Light Source Movement` :`NewTime` (stale _output_get) :!label _label)
              (:`Update`
                (`TimelineComponent.SetPlayRate` (`self.Light Source Movement`) 0.5) ; Destroy connection if system time is used
                (`self.K2_SetActorRotation` (`self.LightSource`) (`KismetMathLibrary.MakeRotator` 0.0 _sun_pitch _sun_yaw) false)
                (`/Game/Environment/Sky/BP_Sky_Sphere_My.UpdateSunDirection` (`self.SkySphere`)))))
          (:`then_1`
            (bind _output_get (set `self.NewTime` 12.0 :!label _label_2))
            (goto _label :!via `SetNewTime`))))
      (:`B`
        (`|ExecutionSequence`
          (:`then_0`
            (goto _label :!via `Stop`))
          (:`then_1`
            (goto _label_2)))))))

(fn `UserConstructionScript`)